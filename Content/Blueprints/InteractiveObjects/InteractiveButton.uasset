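; InteractiveButton is an interactive button that highlights on hover and notifies a listener when used.
; Hover, unhover and use set the mesh's Color material parameter to yellow, white and green.
; On use it calls OnButtonPressedMessage on its Listener if that implements ButtonListenerInterface, so it needs no knowledge of the listener's class.
; Pickup, drop and drag are stubs returning false.
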(fn `CanPickup`
  (returns (Return :type Boolean))
  (return false))

(fn `OnDrag`
  (params (Interactor :type "/Game/Blueprints/Components/WorldInteractor Object Reference"))
  (returns (Return :type Boolean))
  (return false))

(fn `OnDragEnd`
  (params (Interactor :type "/Game/Blueprints/Components/WorldInteractor Object Reference"))
  (returns (Return :type Boolean))
  (return false))

(fn `OnDragStart`
  (params (Interactor :type "/Game/Blueprints/Components/WorldInteractor Object Reference"))
  (returns (Return :type Boolean))
  (return false))

(fn `OnDrop`
  (params (Interactor :type "/Game/Blueprints/Components/WorldInteractor Object Reference"))
  (returns (Return :type Boolean))
  (return false))

(fn `OnHover`
  (params (Interactor :type "/Game/Blueprints/Components/WorldInteractor Object Reference"))
  (returns (Return :type Boolean))
  (`MeshComponent.SetVectorParameterValueOnMaterials` (`self.StaticMeshComponent`) "Color" (1.0 1.0 0.0))
  (return false))

(fn `OnPickup`
  (params (Interactor :type "/Game/Blueprints/Components/WorldInteractor Object Reference"))
  (returns (Return :type Boolean))
  (return false))

(fn `OnUnhover`
  (params (Interactor :type "/Game/Blueprints/Components/WorldInteractor Object Reference"))
  (returns (Return :type Boolean))
  (`MeshComponent.SetVectorParameterValueOnMaterials` (`self.StaticMeshComponent`) "Color" (1.0 1.0 1.0))
  (return false))

(fn `OnUse`
  (params (Interactor :type "/Game/Blueprints/Components/WorldInteractor Object Reference"))
  (returns (Return :type Boolean))
  (`MeshComponent.SetVectorParameterValueOnMaterials` (`self.StaticMeshComponent`) "Color" (0.0 1.0 0.0))
  (if (`KismetSystemLibrary.DoesImplementInterface` (`self.Listener`) "/Game/Blueprints/Interfaces/ButtonListenerInterface.ButtonListenerInterface_C")
    (message `/Game/Blueprints/Interfaces/ButtonListenerInterface.OnButtonPressed` (`self.Listener`)))
  (return false))

(fn `UserConstructionScript`)