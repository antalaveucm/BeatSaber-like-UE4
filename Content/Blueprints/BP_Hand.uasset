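; BP_Hand is a tracked hand actor that derives a grab pose from two trackers.
; Each Tick, it copies both tracker poses, expressed in TrackerOrigin's unscaled space, onto MainPart and SecondPart as relative transforms.
; GrabStrength is one minus the clamped dot product of the parts' Z axes, rising from aligned to perpendicular.
; That value drives the Hand_AnimBP instance cached at BeginPlay.
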(event `self.ReceiveBeginPlay`
  (bind _ashand_anim_bp (cast `/Game/Extras/Hands/Hand_AnimBP` (`SkeletalMeshComponent.GetAnimInstance` (`self.SkeletalMesh`))))
  (set `self.HandAnimCast` _ashand_anim_bp))

(event `self.ReceiveTick`
  (params (DeltaSeconds :type "Float (single-precision)"))
  (`self.UpdateTracking`)
  (set `/Game/Extras/Hands/Hand_AnimBP.GrabStrength` (- 1.0 (`KismetMathLibrary.FClamp` (`KismetMathLibrary.Dot_VectorVector` (`KismetMathLibrary.TransformDirection` (`SceneComponent.K2_GetComponentToWorld` (`self.MainPart`)) (0.0 0.0 1.0)) (`KismetMathLibrary.TransformDirection` (`SceneComponent.K2_GetComponentToWorld` (`self.SecondPart`)) (0.0 0.0 1.0))))) (`self.HandAnimCast`)))

(fn `SetPartPosition`
  (params (HandPart :type "SceneComponent Object Reference") (TrackerOrigin :type "Actor Object Reference") (PartTracker :type "Actor Object Reference"))
  (bind _returnvalue (`KismetMathLibrary.MakeTransform` (.location (`self.GetTransform` TrackerOrigin)) (.rotation (`self.GetTransform` TrackerOrigin))))
  (`SceneComponent.K2_SetRelativeLocationAndRotation` HandPart (`KismetMathLibrary.InverseTransformLocation` _returnvalue (`self.K2_GetActorLocation` PartTracker)) (`KismetMathLibrary.InverseTransformRotation` _returnvalue (`self.K2_GetActorRotation` PartTracker)) false false))

(fn `UpdateTracking`
  (`self.SetPartPosition` (`self.MainPart`) (`self.TrackerOrigin`) (`self.MainTracker`))
  (`self.SetPartPosition` (`self.SecondPart`) (`self.TrackerOrigin`) (`self.SecondTracker`)))

(fn `UserConstructionScript`)