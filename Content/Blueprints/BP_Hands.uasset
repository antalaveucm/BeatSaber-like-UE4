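; BP_Hands drives a pair of tracked hands that pick up, drop and use objects in the world.
; Each tick it converts left and right tracker transforms into the tracker origin's unscaled space and applies them as relative hand transforms.
; Touch (left) and Grasp (right) presses tint that hand's sphere green and toggle its world interactor between dropping and pickup, falling back to using the hovered object.
; A debug function toggles cube visibility.
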(event `self.ReceiveTick`
  (params (DeltaSeconds :type "Float (single-precision)"))
  (`self.UpdateTracking`))

(event `InputTouch`
  (params (Location :type "Vector Structure") (FingerIndex :type "ETouchIndex Enum"))
  (bind _sphere_l (`self.Sphere_L`))
  (:`Pressed`
    (`MeshComponent.SetVectorParameterValueOnMaterials` _sphere_l "Color" (0.0 1.0 0.0))
    (`self.InteractWithWorld` (`self.WorldInteractor_L`)))
  (:`Released`
    (`MeshComponent.SetVectorParameterValueOnMaterials` _sphere_l "Color" (1.0 1.0 1.0))))

(event `InputAction|Grasp`
  (params (Key :type "Key Structure"))
  (bind _sphere_r (`self.Sphere_R`))
  (:`Pressed`
    (`MeshComponent.SetVectorParameterValueOnMaterials` _sphere_r "Color" (0.0 1.0 0.0))
    (`self.InteractWithWorld` (`self.WorldInteractor_R`)))
  (:`Released`
    (`MeshComponent.SetVectorParameterValueOnMaterials` _sphere_r "Color" (1.0 1.0 1.0))))

(fn `InteractWithWorld`
  (params (Interactor :type "/Game/Blueprints/Components/WorldInteractor Object Reference"))
  (`/Engine/EditorBlueprintResources/StandardMacros.IsValid` (`/Game/Blueprints/Components/WorldInteractor.PickedUpObject` Interactor)
    (:`Is Valid`
      (`/Game/Blueprints/Components/WorldInteractor.Drop` Interactor))
    (:`Is Not Valid`
      (`/Game/Blueprints/Components/WorldInteractor.Pickup` Interactor)
      (`/Engine/EditorBlueprintResources/StandardMacros.IsValid` (`/Game/Blueprints/Components/WorldInteractor.PickedUpObject` Interactor)
        (:`Is Not Valid`
          (`/Engine/EditorBlueprintResources/StandardMacros.IsValid` (`/Game/Blueprints/Components/WorldInteractor.HoveredObject` Interactor)
            (:`Is Valid`
              (`/Game/Blueprints/Components/WorldInteractor.UseHoveredObject` Interactor))))))))

(fn `SetDebug`
  (params (Value :type Boolean))
  (returns (Return :type Boolean))
  (bind _returnvalue (not Value))
  (`SceneComponent.SetHiddenInGame` (`self.Cube_L`) _returnvalue false)
  (`SceneComponent.SetHiddenInGame` (`self.Cube_R`) _returnvalue false)
  (return false))

(fn `SetHandPosition`
  (params (Hand :type "SceneComponent Object Reference") (TrackerOrigin :type "Actor Object Reference") (HandTracker :type "Actor Object Reference"))
  (bind _returnvalue (`KismetMathLibrary.MakeTransform` (.location (`self.GetTransform` TrackerOrigin)) (.rotation (`self.GetTransform` TrackerOrigin))))
  (`SceneComponent.K2_SetRelativeLocationAndRotation` Hand (`KismetMathLibrary.InverseTransformLocation` _returnvalue (`self.K2_GetActorLocation` HandTracker)) (`KismetMathLibrary.InverseTransformRotation` _returnvalue (`self.K2_GetActorRotation` HandTracker)) false false))

(fn `UpdateTracking`
  (`self.SetHandPosition` (`self.Hand_L`) (`self.TrackerOrigin`) (`self.Tracker_L`))
  (`self.SetHandPosition` (`self.Hand_R`) (`self.TrackerOrigin`) (`self.Tracker_R`)))

(fn `UserConstructionScript`)