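; Walk-in-place VR locomotion actor that moves its scene root horizontally along the CameraPawn's VR camera heading.
; The Gravity vector input triggers a step when its magnitude drops below a threshold, with StepLock blocking repeats until it rises back.
; WalkForward and WalkBackwards presses add small steps either way.
; All movement goes through StepForward, which offsets the root without sweeping for collision.
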(event `InputVectorAxis|Gravity`
  (params (AxisValue :type "Vector Structure"))
  (bind _returnvalue (`KismetMathLibrary.VSize` AxisValue))
  (bind _gravitythreshold (`self.GravityThreshold`))
  ;[1 1 1] Walk-in-place technique
  (if (`self.StepLock`)
    (if (>= _returnvalue _gravitythreshold)
      (set `self.StepLock` false))
    (elif (< _returnvalue _gravitythreshold)
      (set `self.StepLock` true)
      (`self.StepForward` (`self.StepLength`)))))

(event `InputAction|WalkForward`
  (params (Key :type "Key Structure"))
  (:`Pressed`
    (`self.StepForward` (`self.SmallStepLength`))))

(event `InputAction|WalkBackwards`
  (params (Key :type "Key Structure"))
  (:`Pressed`
    (`self.StepForward` (* (`self.SmallStepLength`) -1.0))))

(fn `StepForward`
  (params (Length :type "Float (double-precision)"))
  (`SceneComponent.K2_SetWorldLocation` (`self.DefaultSceneRoot`) (+ (`SceneComponent.K2_GetComponentLocation` (`self.DefaultSceneRoot`)) (* (`KismetMathLibrary.Normal` (`KismetMathLibrary.ProjectVectorOnToPlane` (`KismetMathLibrary.GetForwardVector` (`SceneComponent.K2_GetComponentRotation` (`/Game/Blueprints/BP_AURCameraPawn.VRCamera` (`self.CameraPawn`)))) (0.0 0.0 1.0))) Length)) false false))

(fn `UserConstructionScript`)