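; VR camera root actor that switches the view between standing and crouching heights.
; It applies the standing height on BeginPlay, and the Crouch input toggles between the two heights using an IsCrouched flag.
; SetCameraHeight moves DefaultSceneRoot instantly to the given relative Z, zeroing X and Y, with no sweep or interpolation.
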(event `self.ReceiveBeginPlay`
  (`self.SetCameraHeight` (`self.StandingHeight`)))

(event `InputAction|Crouch`
  (params (Key :type "Key Structure"))
  (:`Pressed`
    (if (`self.IsCrouched`)
      (`self.SetCameraHeight` (`self.StandingHeight`))
      (set `self.IsCrouched` false)
      (else
        (`self.SetCameraHeight` (`self.CrouchingHeight`))
        (set `self.IsCrouched` true)))))

(fn `SetCameraHeight`
  (params (Z :type "Float (double-precision)"))
  (`SceneComponent.K2_SetRelativeLocation` (`self.DefaultSceneRoot`) (`KismetMathLibrary.MakeVector` 0.0 0.0 Z) false false))

(fn `UserConstructionScript`)