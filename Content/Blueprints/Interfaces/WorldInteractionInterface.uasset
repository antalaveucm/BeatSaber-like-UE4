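; WorldInteractionInterface is a Blueprint interface for objects in the world that an interactor can act on.
; It declares events for hover and unhover, use, pickup and drop, and drag start, drag and drag end, each receiving the Interactor.
; A CanPickup query lets an object report whether it can be picked up; every function body here returns false as a stub.
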(fn `CanPickup`
  (returns (Return :type Boolean))
  (return false))

(fn `OnDrag`
  (params (Interactor :type "/Game/Blueprints/Components/WorldInteractor Object Reference"))
  (returns (Return :type Boolean))
  (return false))

(fn `OnDragEnd`
  (params (Interactor :type "/Game/Blueprints/Components/WorldInteractor Object Reference"))
  (returns (Return :type Boolean))
  (return false))

(fn `OnDragStart`
  (params (Interactor :type "/Game/Blueprints/Components/WorldInteractor Object Reference"))
  (returns (Return :type Boolean))
  (return false))

(fn `OnDrop`
  (params (Interactor :type "/Game/Blueprints/Components/WorldInteractor Object Reference"))
  (returns (Return :type Boolean))
  (return false))

(fn `OnHover`
  (params (Interactor :type "/Game/Blueprints/Components/WorldInteractor Object Reference"))
  (returns (Return :type Boolean))
  (return false))

(fn `OnPickup`
  (params (Interactor :type "/Game/Blueprints/Components/WorldInteractor Object Reference"))
  (returns (Return :type Boolean))
  (return false))

(fn `OnUnhover`
  (params (Interactor :type "/Game/Blueprints/Components/WorldInteractor Object Reference"))
  (returns (Return :type Boolean))
  (return false))

(fn `OnUse`
  (params (Interactor :type "/Game/Blueprints/Components/WorldInteractor Object Reference"))
  (returns (Return :type Boolean))
  (return false))