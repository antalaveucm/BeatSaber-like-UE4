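; BP_Menu is an in-world difficulty menu actor that starts the cube spawning game when one of its three boxes is overlapped.
; Each box's overlap destroys the menu, sets its Difficulty to one of three levels, then finds BP_CubeSpawner with GetActorOfClass and sets its StartGame flag.
; Difficulty is not passed to the spawner here, and the second and third boxes also print the StartGame value.
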(event `self.Box.OnComponentBeginOverlap`
  (params (OverlappedComponent :type "PrimitiveComponent Object Reference") (OtherActor :type "Actor Object Reference") (OtherComp :type "PrimitiveComponent Object Reference") (OtherBodyIndex :type Integer) (bFromSweep :type Boolean) (SweepResult :type "HitResult Structure (by ref)"))
  (`self.K2_DestroyActor`)
  (set `self.Difficulty` 1)
  (bind _returnvalue (`GameplayStatics.GetActorOfClass` "/Game/Blueprints/BP_CubeSpawner.BP_CubeSpawner_C"))
  (set `/Game/Blueprints/BP_CubeSpawner.StartGame` true _returnvalue))

(event `self.Box1.OnComponentBeginOverlap`
  (params (OverlappedComponent :type "PrimitiveComponent Object Reference") (OtherActor :type "Actor Object Reference") (OtherComp :type "PrimitiveComponent Object Reference") (OtherBodyIndex :type Integer) (bFromSweep :type Boolean) (SweepResult :type "HitResult Structure (by ref)"))
  (`self.K2_DestroyActor`)
  (set `self.Difficulty` 2)
  (bind _returnvalue (`GameplayStatics.GetActorOfClass` "/Game/Blueprints/BP_CubeSpawner.BP_CubeSpawner_C"))
  (bind _output_get (set `/Game/Blueprints/BP_CubeSpawner.StartGame` true _returnvalue))
  (`KismetSystemLibrary.PrintString` (`KismetStringLibrary.Conv_BoolToString` _output_get)))

(event `self.Box2.OnComponentBeginOverlap`
  (params (OverlappedComponent :type "PrimitiveComponent Object Reference") (OtherActor :type "Actor Object Reference") (OtherComp :type "PrimitiveComponent Object Reference") (OtherBodyIndex :type Integer) (bFromSweep :type Boolean) (SweepResult :type "HitResult Structure (by ref)"))
  (`self.K2_DestroyActor`)
  (set `self.Difficulty` 3)
  (bind _returnvalue (`GameplayStatics.GetActorOfClass` "/Game/Blueprints/BP_CubeSpawner.BP_CubeSpawner_C"))
  (bind _output_get (set `/Game/Blueprints/BP_CubeSpawner.StartGame` true _returnvalue))
  (`KismetSystemLibrary.PrintString` (`KismetStringLibrary.Conv_BoolToString` _output_get)))

(fn `UserConstructionScript`)