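; BP_AURCameraPawn is an AR camera pawn with a first-person camera and a video screen background.
; Each tick it sets the root's relative rotation from the device orientation, ignoring position.
; A custom FOV event updates the camera and resizes the video screen to match.
; Debug events and a SetDebug function toggle the visibility of that video screen.
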(event `self.ReceiveBeginPlay`
  (set `self.VRCamera` (`self.FirstPersonCamera`)))

(event `self.ReceiveTick`
  (params (DeltaSeconds :type "Float (single-precision)"))
  (`self.UpdateTracking`))

(event `/Game/Blueprints/BPi_CameraSettings.SetCustomFOV`
  (params (fov :type "Float (single-precision)"))
  (`CameraComponent.SetFieldOfView` (`self.FirstPersonCamera`) fov)
  (`AURVideoScreenBackground.SetSizeForFOV` (`self.AURVideoScreenBackgroundComponent`) fov))

(event `DisableDebug`
  (`SceneComponent.SetHiddenInGame` (`self.AURVideoScreenBackgroundComponent`) true false))

(event `EnableDebug`
  (`SceneComponent.SetHiddenInGame` (`self.AURVideoScreenBackgroundComponent`) false false))

(fn `SetDebug`
  (params (Value :type Boolean))
  (returns (Return :type Boolean))
  (`SceneComponent.SetHiddenInGame` (`self.AURVideoScreenBackgroundComponent`) (not Value) false)
  (return false))

(fn `UpdateTracking`
  (`SceneComponent.K2_SetRelativeRotation` (`self.DefaultSceneRoot`) (`HeadMountedDisplayFunctionLibrary.GetOrientationAndPosition`) false false))

(fn `UserConstructionScript`)