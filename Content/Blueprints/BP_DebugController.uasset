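; BP_DebugController is an actor that switches debug messaging on and off for a set of actors.
; OnButtonPressed flips the Debugging flag, passes the new state to each entry in ActorArray through SetDebugMessage, and returns false.
; While debugging is on, any key press prints that key's display name on screen in red.
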(event `Key|AnyKey` :consume false
  (params (Key :type "Key Structure"))
  (:`Pressed`
    (if (`self.Debugging`)
      (`KismetSystemLibrary.PrintString` (`KismetTextLibrary.Conv_TextToString` (`KismetInputLibrary.Key_GetDisplayName` Key)) true false (struct :`R` 1.0 :`A` 1.0) 3.0))))

(fn `OnButtonPressed`
  (returns (Return :type Boolean))
  (bind _output_get (set `self.Debugging` (not (`self.Debugging`))))
  (for _array_element (`self.ActorArray`)
    (message `/Game/Blueprints/Interfaces/DebugInterface.SetDebug` _array_element _output_get))
  (return false))

(fn `UserConstructionScript`)