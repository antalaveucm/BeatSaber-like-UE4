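; BP_CubeSpawner is an actor that repeatedly spawns BP_Cube actors at its own location once the game has started.
; From BeginPlay, CheckStartGame polls the StartGame flag by calling itself after a short delay until it is true.
; It then starts a looping timer on SpawnCube, whose random interval of a few seconds is picked once, when the timer is set.
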(event `CheckStartGame`
  (if (== (`self.StartGame`) true)
    (`KismetSystemLibrary.K2_SetTimer` null "SpawnCube" (`KismetMathLibrary.RandomFloatInRange` 2.0 4.0) true)
    (else
      (`KismetSystemLibrary.Delay` 0.5)
      (`self.CheckStartGame`))))

(event `self.ReceiveBeginPlay`
  (`self.CheckStartGame`))

(event `self.ReceiveTick`
  (params (DeltaSeconds :type "Float (single-precision)")))

(fn `SpawnCube`
  (`|SpawnActorFromClass` "/Game/Blueprints/BP_Cube.BP_Cube_C" (`KismetMathLibrary.Conv_VectorToTransform` (`self.K2_GetActorLocation`)) "Undefined" "OverrideRootScale" null null))

(fn `UserConstructionScript`)